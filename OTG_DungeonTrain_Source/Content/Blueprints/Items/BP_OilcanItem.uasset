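; Oilcan pickup item that raises the oilcan count and lowers the AttackSpeed value when collected.
; Overlap toggles a widget's visibility, and Interact calls AddOilCan, then destroys the actor.
; AddOilCan increments the count in the globalVariables game instance and recomputes AttackSpeed from it as a linear reduction with no clamp.
; The construction script sets the Paper2D sprite from the Item data.
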(event Collision|EventActorBeginOverlap
  (params (OtherActor :type Actor%20Object%20Reference))
  (Rendering|SetVisibility (Variables|Default|GetWidget) true false))

(event Collision|EventActorEndOverlap
  (params (OtherActor :type Actor%20Object%20Reference))
  (Rendering|SetVisibility (Variables|Default|GetWidget) false false))

(event EventInteract
  (CallFunction|AddOilCan)
  (Actor|DestroyActor))

(fn ConstructionScript
  (Rendering|Components|Sprite|SetSprite (Variables|Default|GetPaperSprite) (.Sprite (Utilities|Struct|BreakItemStructure (Variables|Default|GetItem)))))

(fn AddOilCan
  (bind _asglobal_variables (Utilities|Casting|CastToglobalVariables (Game|GetGameInstance)))
  (bind _output_get (Variables|/Game/Blueprints/globalVariables.globalVariables_C|Setcount_Oilcan _asglobal_variables (+ (Variables|/Game/Blueprints/globalVariables.globalVariables_C|Getcount_Oilcan _asglobal_variables) 1)))
  (Variables|/Game/Blueprints/globalVariables.globalVariables_C|SetattackSpeed _asglobal_variables (- 1.0 (* _output_get 0.05))))