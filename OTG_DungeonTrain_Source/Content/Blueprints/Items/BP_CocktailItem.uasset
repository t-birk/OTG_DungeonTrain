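; BP_CocktailItem is a 2D pickup item whose stacks raise health regeneration.
; On Interact it increments the cocktail count in the globalVariables game instance, sets HealthRegen from that count, then destroys itself.
; Overlap events toggle a widget's visibility, ignoring actors tagged as light or heavy attacks.
; The construction script sets the Paper2D sprite from the Item data.
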(event Collision|EventActorBeginOverlap
  (params (OtherActor :type Actor%20Object%20Reference))
  (if (not (Actor|ActorHasTag OtherActor "lightAttack"))
    (if (not (Actor|ActorHasTag OtherActor "heavyAttack"))
      (Rendering|SetVisibility (Variables|Default|GetWidget) true false))))

(event Collision|EventActorEndOverlap
  (params (OtherActor :type Actor%20Object%20Reference))
  (if (not (Actor|ActorHasTag OtherActor "lightAttack"))
    (if (not (Actor|ActorHasTag OtherActor "heavyAttack"))
      (Rendering|SetVisibility (Variables|Default|GetWidget) false false))))

(event EventInteract
  (CallFunction|AddCocktail)
  (Actor|DestroyActor))

(fn ConstructionScript
  (Rendering|Components|Sprite|SetSprite (Variables|Default|GetPaperSprite) (.Sprite (Utilities|Struct|BreakItemStructure (Variables|Default|GetItem)))))

(fn AddCocktail
  (bind _asglobal_variables (Utilities|Casting|CastToglobalVariables (Game|GetGameInstance)))
  (bind _output_get (Variables|/Game/Blueprints/globalVariables.globalVariables_C|Setcount_Cocktail _asglobal_variables (+ (Variables|/Game/Blueprints/globalVariables.globalVariables_C|Getcount_Cocktail _asglobal_variables) 1)))
  (Variables|/Game/Blueprints/globalVariables.globalVariables_C|SethealthRegen _asglobal_variables (Math|Conversions|ToFloat(Integer) (* _output_get 1))))