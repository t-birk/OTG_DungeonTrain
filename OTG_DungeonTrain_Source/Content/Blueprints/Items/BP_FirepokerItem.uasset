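; Pickup item actor for a firepoker that raises the player's attack power when collected.
; Overlap shows or hides a widget, and the construction script sets the paper sprite from the item's data.
; Interacting increments the firepoker count in the globalVariables game instance, recalculates AttackPower as that count plus one, then destroys the actor.
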(event Collision|EventActorBeginOverlap
  (params (OtherActor :type Actor%20Object%20Reference))
  (Rendering|SetVisibility (Variables|Default|GetWidget) true false))

(event Collision|EventActorEndOverlap
  (params (OtherActor :type Actor%20Object%20Reference))
  (Rendering|SetVisibility (Variables|Default|GetWidget) false false))

(event EventInteract
  (CallFunction|AddFirepoker)
  (Actor|DestroyActor))

(fn ConstructionScript
  (Rendering|Components|Sprite|SetSprite (Variables|Default|GetPaperSprite) (.Sprite (Utilities|Struct|BreakItemStructure (Variables|Default|GetItem)))))

(fn AddFirepoker
  (bind _asglobal_variables (Utilities|Casting|CastToglobalVariables (Game|GetGameInstance))
    (:then
      (bind _output_get (Variables|/Game/Blueprints/globalVariables.globalVariables_C|Setcount_Firepoker _asglobal_variables (+ (Variables|/Game/Blueprints/globalVariables.globalVariables_C|Getcount_Firepoker _asglobal_variables) 1)))
      (Variables|/Game/Blueprints/globalVariables.globalVariables_C|SetattackPower _asglobal_variables (Math|Conversions|ToFloat(Integer) (+ (* _output_get 1) 1)))
      (Development|PrintString "Added"))
    (:CastFailed
      (Development|PrintString "cast failed"))))