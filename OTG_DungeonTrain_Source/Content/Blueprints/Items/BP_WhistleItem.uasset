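; BP_WhistleItem is an interactable whistle pickup that raises the player's total dash count.
; Its construction script sets the Paper2D sprite from the Item data, and actor overlap toggles a widget's visibility.
; On Interact it increments the whistle count in the globalVariables Game Instance, derives the dash total from that count plus a fixed base, then destroys itself.
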(event Collision|EventActorBeginOverlap
  (params (OtherActor :type Actor%20Object%20Reference))
  (Rendering|SetVisibility (Variables|Default|GetWidget) true false))

(event Collision|EventActorEndOverlap
  (params (OtherActor :type Actor%20Object%20Reference))
  (Rendering|SetVisibility (Variables|Default|GetWidget) false false))

(event EventInteract
  (CallFunction|AddWhistle)
  (Actor|DestroyActor))

(fn ConstructionScript
  (Rendering|Components|Sprite|SetSprite (Variables|Default|GetPaperSprite) (.Sprite (Utilities|Struct|BreakItemStructure (Variables|Default|GetItem)))))

(fn AddWhistle
  (bind _asglobal_variables (Utilities|Casting|CastToglobalVariables (Game|GetGameInstance))
    (:then
      (bind _output_get (Variables|/Game/Blueprints/globalVariables.globalVariables_C|Setcount_Whistle _asglobal_variables (+ (Variables|/Game/Blueprints/globalVariables.globalVariables_C|Getcount_Whistle _asglobal_variables) 1)))
      (Variables|/Game/Blueprints/globalVariables.globalVariables_C|SetdashCountTotal _asglobal_variables (+ _output_get 2))
      (Development|PrintString "Added"))
    (:CastFailed
      (Development|PrintString "cast failed"))))