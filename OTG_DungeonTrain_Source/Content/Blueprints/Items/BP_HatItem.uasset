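; BP_HatItem is an interactable hat pickup that raises the player's maximum health.
; Its construction script sets the sprite from its Item data, and actor overlap shows or hides a widget.
; On Interact it increments the hat count in the globalVariables game instance, recalculates max health from that count, then destroys itself.
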(event Collision|EventActorBeginOverlap
  (params (OtherActor :type Actor%20Object%20Reference))
  (Rendering|SetVisibility (Variables|Default|GetWidget) true false))

(event Collision|EventActorEndOverlap
  (params (OtherActor :type Actor%20Object%20Reference))
  (Rendering|SetVisibility (Variables|Default|GetWidget) false false))

(event EventInteract
  (CallFunction|AddHat)
  (Actor|DestroyActor))

(fn ConstructionScript
  (Rendering|Components|Sprite|SetSprite (Variables|Default|GetPaperSprite) (.Sprite (Utilities|Struct|BreakItemStructure (Variables|Default|GetItem)))))

(fn AddHat
  (bind _asglobal_variables (Utilities|Casting|CastToglobalVariables (Game|GetGameInstance)))
  (bind _output_get (Variables|/Game/Blueprints/globalVariables.globalVariables_C|Setcount_Hat _asglobal_variables (+ (Variables|/Game/Blueprints/globalVariables.globalVariables_C|Getcount_Hat _asglobal_variables) 1)))
  (Variables|/Game/Blueprints/globalVariables.globalVariables_C|SetmaxHealth _asglobal_variables (+ (* _output_get 4) 20)))