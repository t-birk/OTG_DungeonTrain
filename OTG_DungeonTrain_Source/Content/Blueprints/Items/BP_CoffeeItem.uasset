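; BP_CoffeeItem is a collectible coffee pickup that permanently counts toward a player movement speed bonus.
; Its sprite is set from the Item data in the construction script, and a widget shows while an actor overlaps it.
; Interact increments the coffee count in the globalVariables GameInstance, recalculates the linear speed multiplier, applies it to the player character's MaxWalkSpeed, then destroys the pickup.
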(event Collision|EventActorBeginOverlap
  (params (OtherActor :type Actor%20Object%20Reference))
  (Rendering|SetVisibility (Variables|Default|GetWidget) true false))

(event Collision|EventActorEndOverlap
  (params (OtherActor :type Actor%20Object%20Reference))
  (Rendering|SetVisibility (Variables|Default|GetWidget) false false))

(event EventInteract
  (CallFunction|AddCoffee)
  (Actor|DestroyActor))

(fn ConstructionScript
  (Rendering|Components|Sprite|SetSprite (Variables|Default|GetPaperSprite) (.Sprite (Utilities|Struct|BreakItemStructure (Variables|Default|GetItem)))))

(fn AddCoffee
  (bind _asglobal_variables (Utilities|Casting|CastToglobalVariables (Game|GetGameInstance)))
  (bind _output_get (Variables|/Game/Blueprints/globalVariables.globalVariables_C|Setcount_Coffee _asglobal_variables (+ (Variables|/Game/Blueprints/globalVariables.globalVariables_C|Getcount_Coffee _asglobal_variables) 1)))
  (Variables|/Game/Blueprints/globalVariables.globalVariables_C|SetmoveSpeedBonus _asglobal_variables (+ (* (Math|Conversions|ToFloat(Integer) _output_get) 0.1) 1.0))
  (Variables|/Script/Engine.CharacterMovementComponent|SetMaxWalkSpeed (Variables|/Script/Engine.Character|GetCharacterMovement (Game|GetPlayerCharacter 0)) (* (Variables|/Game/Blueprints/globalVariables.globalVariables_C|GetmoveSpeedBonus _asglobal_variables) 4e+02)))