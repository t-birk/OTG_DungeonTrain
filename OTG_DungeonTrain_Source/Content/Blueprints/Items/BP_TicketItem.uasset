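; BP_TicketItem is a collectible ticket pickup that raises the dodge percentage.
; Its construction script sets the Paper2D sprite from its Item data, and a widget shows while another actor overlaps it.
; On Interact it increments the ticket count in the globalVariables game instance, recalculates DodgePercent linearly from that count, then destroys itself.
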(event Collision|EventActorBeginOverlap
  (params (OtherActor :type Actor%20Object%20Reference))
  (Rendering|SetVisibility (Variables|Default|GetWidget) true false))

(event Collision|EventActorEndOverlap
  (params (OtherActor :type Actor%20Object%20Reference))
  (Rendering|SetVisibility (Variables|Default|GetWidget) false false))

(event EventInteract
  (CallFunction|AddTicket)
  (Actor|DestroyActor))

(fn ConstructionScript
  (Rendering|Components|Sprite|SetSprite (Variables|Default|GetPaperSprite) (.Sprite (Utilities|Struct|BreakItemStructure (Variables|Default|GetItem)))))

(fn AddTicket
  (bind _asglobal_variables (Utilities|Casting|CastToglobalVariables (Game|GetGameInstance)))
  (bind _output_get (Variables|/Game/Blueprints/globalVariables.globalVariables_C|Setcount_Ticket _asglobal_variables (+ (Variables|/Game/Blueprints/globalVariables.globalVariables_C|Getcount_Ticket _asglobal_variables) 1)))
  (Variables|/Game/Blueprints/globalVariables.globalVariables_C|SetdodgePercent _asglobal_variables (* _output_get 0.01)))