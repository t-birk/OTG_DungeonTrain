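; Shop pedestal that sells one of eight random upgrade items for gold, with a randomized price that scales with level count.
; BeginPlay picks the item's sprite and name; overlap toggles the prompt and price, ignoring attack-tagged actors.
; Interact deducts gold from the globalVariables GameInstance and calls the Add function on the matching item actor, found via GetActorOfClass.
; The pedestal then destroys itself with explosion effects.
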(event EventBeginPlay
  (Variables|Default|Setavailable_Item "")
  (Variables|Default|SetrandomSpawnInteger 0)
  (bind _asglobal_variables (Utilities|Casting|CastToglobalVariables (Game|GetGameInstance)))
  (Variables|Default|SetpurchaseCost (+ (* (Variables|/Game/Blueprints/globalVariables.globalVariables_C|GetlevelCount _asglobal_variables) (Math|Random|RandomFloatinRange 0.5 2.5)) 20))
  (bind _output_get (Variables|Default|SetrandomSpawnInteger (Math|Random|RandomIntegerinRange 1 8)))
  (if (== _output_get 1)
    (Rendering|Components|Sprite|SetSprite (Variables|Default|Getitem) "/Game/TopDown/Blueprints/UI/Inventory/Images/Train_Whistle_-_Dash_Charge_Sprite.Train_Whistle_-_Dash_Charge_Sprite")
    (Variables|Default|Setavailable_Item "Whistle")
    (elif (== _output_get 2)
      (Rendering|Components|Sprite|SetSprite (Variables|Default|Getitem) "/Game/TopDown/Blueprints/UI/Inventory/Images/Cocktail_-_Regen_Sprite.Cocktail_-_Regen_Sprite")
      (Variables|Default|Setavailable_Item "Cocktail")
      (elif (== _output_get 3)
        (Rendering|Components|Sprite|SetSprite (Variables|Default|Getitem) "/Game/TopDown/Blueprints/UI/Inventory/Images/Coffee_-_Move_Speed_Sprite.Coffee_-_Move_Speed_Sprite")
        (Variables|Default|Setavailable_Item "Coffee")
        (elif (== _output_get 4)
          (Rendering|Components|Sprite|SetSprite (Variables|Default|Getitem) "/Game/TopDown/Blueprints/UI/Inventory/Images/Firepoker_-_Attack__Sprite.Firepoker_-_Attack__Sprite")
          (Variables|Default|Setavailable_Item "Firepoker")
          (elif (== _output_get 5)
            (Rendering|Components|Sprite|SetSprite (Variables|Default|Getitem) "/Game/TopDown/Blueprints/UI/Inventory/Images/Conductor_Hat_-_Health_Sprite.Conductor_Hat_-_Health_Sprite")
            (Variables|Default|Setavailable_Item "Hat")
            (elif (== _output_get 6)
              (Rendering|Components|Sprite|SetSprite (Variables|Default|Getitem) "/Game/TopDown/Blueprints/UI/Inventory/Images/Oil_Can_-_Attack_Speed_Sprite.Oil_Can_-_Attack_Speed_Sprite")
              (Variables|Default|Setavailable_Item "Oil_can")
              (elif (== _output_get 7)
                (Rendering|Components|Sprite|SetSprite (Variables|Default|Getitem) "/Game/TopDown/Blueprints/UI/Inventory/Images/Ticket_-_Dodge_Chance_Sprite.Ticket_-_Dodge_Chance_Sprite")
                (Variables|Default|Setavailable_Item "Ticket")
                (elif (== _output_get 8)
                  (Rendering|Components|Sprite|SetSprite (Variables|Default|Getitem) "/Game/TopDown/Blueprints/UI/Inventory/Images/Watch_-_Health_Sprite.Watch_-_Health_Sprite")
                  (Variables|Default|Setavailable_Item "Watch")
                  (else
                    (Development|PrintString (Utilities|String|ToString(Integer) _output_get))
                    (Development|PrintString "Thats fucked")))))))))))

(event Collision|EventActorBeginOverlap
  (params (OtherActor :type Actor%20Object%20Reference))
  (if (not (Actor|ActorHasTag OtherActor "lightAttack"))
    (if (not (Actor|ActorHasTag OtherActor "heavyAttack"))
      (Rendering|SetVisibility (Variables|Default|GetPurchase%20Prompt) true false))))

(event Collision|EventActorEndOverlap
  (params (OtherActor :type Actor%20Object%20Reference))
  (if (not (Actor|ActorHasTag OtherActor "lightAttack"))
    (if (not (Actor|ActorHasTag OtherActor "heavyAttack"))
      (Rendering|SetVisibility (Variables|Default|GetPurchase%20Prompt) false false))))

(event EventInteract
  (bind _purchasecost (Variables|Default|GetpurchaseCost))
  (bind _asglobal_variables (Utilities|Casting|CastToglobalVariables (Game|GetGameInstance)))
  (if (>= (Variables|/Game/Blueprints/globalVariables.globalVariables_C|GetgoldMoneyCount _asglobal_variables) _purchasecost)
    (Variables|/Game/Blueprints/globalVariables.globalVariables_C|SetgoldMoneyCount _asglobal_variables (- (Variables|/Game/Blueprints/globalVariables.globalVariables_C|GetgoldMoneyCount _asglobal_variables) _purchasecost))
    (Development|PrintString (Variables|Default|Getavailable_Item))
    (if (Utilities|Enum|Equal(Enum) (Variables|Default|Getavailable_Item) "Whistle")
      (bind _returnvalue (Actor|GetActorOfClass "/Game/TopDown/Blueprints/UI/Inventory/PlaceholderUntilBetterSystem/BP_WhistleItem.BP_WhistleItem_C"))
      (Default|AddWhistle _returnvalue)
      (Actor|DestroyActor :!label _label)
      (bind _returnvalue_2 (Effects|SpawnEmitteratLocation "/Game/StarterContent/Particles/P_Explosion.P_Explosion" (Transformation|GetActorLocation)))
      (Audio|PlaySoundatLocation "/Game/StarterContent/Audio/Explosion01.Explosion01" "0, 0, 0" "0, 0, 0" 1.0 1.0 0.0 0 0 0 0)
      (Utilities|FlowControl|Delay 1.0)
      (Components|Activation|Deactivate _returnvalue_2)
      (elif (Utilities|Enum|Equal(Enum) (Variables|Default|Getavailable_Item) "Cocktail")
        (bind _returnvalue_3 (Actor|GetActorOfClass "/Game/TopDown/Blueprints/UI/Inventory/PlaceholderUntilBetterSystem/BP_CocktailItem.BP_CocktailItem_C"))
        (Default|AddCocktail _returnvalue_3)
        (goto _label)
        (elif (Utilities|Enum|Equal(Enum) (Variables|Default|Getavailable_Item) "Coffee")
          (bind _returnvalue_4 (Actor|GetActorOfClass "/Game/TopDown/Blueprints/UI/Inventory/PlaceholderUntilBetterSystem/BP_CoffeeItem.BP_CoffeeItem_C"))
          (Default|AddCoffee _returnvalue_4)
          (goto _label)
          (elif (Utilities|Enum|Equal(Enum) (Variables|Default|Getavailable_Item) "Firepoker")
            (bind _returnvalue_5 (Actor|GetActorOfClass "/Game/TopDown/Blueprints/UI/Inventory/PlaceholderUntilBetterSystem/BP_FirepokerItem.BP_FirepokerItem_C"))
            (Default|AddFirepoker _returnvalue_5)
            (goto _label)
            (elif (Utilities|Enum|Equal(Enum) (Variables|Default|Getavailable_Item) "Hat")
              (bind _returnvalue_6 (Actor|GetActorOfClass "/Game/TopDown/Blueprints/UI/Inventory/PlaceholderUntilBetterSystem/BP_HatItem.BP_HatItem_C"))
              (Default|AddHat _returnvalue_6)
              (goto _label)
              (elif (Utilities|Enum|Equal(Enum) (Variables|Default|Getavailable_Item) "Oil_can")
                (bind _returnvalue_7 (Actor|GetActorOfClass "/Game/TopDown/Blueprints/UI/Inventory/PlaceholderUntilBetterSystem/BP_OilcanItem.BP_OilcanItem_C"))
                (Default|AddOilCan _returnvalue_7)
                (goto _label)
                (elif (Utilities|Enum|Equal(Enum) (Variables|Default|Getavailable_Item) "Ticket")
                  (bind _returnvalue_8 (Actor|GetActorOfClass "/Game/TopDown/Blueprints/UI/Inventory/PlaceholderUntilBetterSystem/BP_TicketItem.BP_TicketItem_C"))
                  (Default|AddTicket _returnvalue_8)
                  (goto _label)
                  (elif (Utilities|Enum|Equal(Enum) (Variables|Default|Getavailable_Item) "Watch")
                    (bind _returnvalue_9 (Actor|GetActorOfClass "/Game/TopDown/Blueprints/UI/Inventory/PlaceholderUntilBetterSystem/BP_WatchItem.BP_WatchItem_C"))
                    (Default|AddWatch _returnvalue_9)
                    (goto _label)))))))))
    (else
      (Development|PrintString "Broke ass"))))

(fn ConstructionScript)