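; HeavyAttackAOE is an area-of-effect hit actor for a heavy attack against Ember enemies.
; It plays a spike trap sound at its location when spawned.
; On overlap with an enemy_Ember, it applies light fixed damage credited to the player controller.
; It then launches the enemy horizontally away from the player character with a large additive knockback along the normalized direction between them.
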(event EventBeginPlay
  (Audio|PlaySoundatLocation "/Game/Sound/Attack/spike_trap_a.spike_trap_a" (Transformation|GetActorLocation) "0, 0, 0" 1.0 1.0 0.0 0 0 0 0))

(event Collision|EventActorBeginOverlap
  (params (OtherActor :type Actor%20Object%20Reference))
  (bind _asenemy_ember (Utilities|Casting|CastToenemy_Ember OtherActor))
  (Game|Damage|ApplyDamage _asenemy_ember 2.0 (Game|GetPlayerController 0) self)
  (Character|LaunchCharacter _asenemy_ember (* (Math|Vector|Normalize (- (Transformation|GetActorLocation (Game|GetPlayerCharacter 0)) (Transformation|GetActorLocation _asenemy_ember))) "-30000.000000,-30000.000000,0.000000") false false))

(event EventTick
  (params (DeltaSeconds :type Float%20%28single-precision%29)))

(fn ConstructionScript)