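; GreasemanProjectile is a short-lived projectile actor that hits the player character.
; On BeginPlay it adds a projectile movement component and destroys itself after a three-second delay.
; When its collision component overlaps an actor whose class is exactly BP_TopDownCharacter, it calls DamagePlayer and destroys itself.
; DamagePlayer is a placeholder that only prints debug text and applies no actual damage.
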(event OnComponentBeginOverlap(ProjCollision)
  (params (OverlappedComponent :type Primitive%20Component%20Object%20Reference) (OtherActor :type Actor%20Object%20Reference) (OtherComp :type Primitive%20Component%20Object%20Reference) (OtherBodyIndex :type Integer) (bFromSweep :type Boolean) (SweepResult :type Hit%20Result%20Structure%20%28by%20ref%29))
  (if (== (Utilities|GetClass OtherActor) "/Game/TopDown/Blueprints/BP_TopDownCharacter.BP_TopDownCharacter_C")
    (CallFunction|DamagePlayer)
    (Actor|DestroyActor)))

(event EventBeginPlay
  (AddComponent|AddProjectileMovementComponent)
  (Utilities|FlowControl|Delay 3.0)
  (Actor|DestroyActor))

(event Collision|EventActorBeginOverlap
  (params (OtherActor :type Actor%20Object%20Reference)))

(event EventTick
  (params (DeltaSeconds :type Float%20%28single-precision%29)))

(fn ConstructionScript)

(fn DamagePlayer
  (Development|PrintText "Player Damage"))