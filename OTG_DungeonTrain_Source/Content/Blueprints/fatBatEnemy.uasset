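; Fat bat enemy character with a flipbook sprite that chases the player, with health scaled by the level count.
; Player overlap deals damage immediately, then on a looping timer cleared shortly after overlap ends.
; Hits flash it red, play a sound and briefly slow it.
; Death decrements the global enemy count and may drop an item through chained re-rolled random checks, whose whistle branch can never succeed.
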(event Custom|DealDamage
  (Game|Damage|ApplyDamage (stale Collision|EventActorBeginOverlap _asbp_top_down_character) 1.0 (Game|GetPlayerController 0) self))

(event EventBeginPlay
  (bind _asglobal_variables (Utilities|Casting|CastToglobalVariables (Game|GetGameInstance)))
  (Variables|Default|SetHealth (* (Variables|/Game/Blueprints/globalVariables.globalVariables_C|GetlevelCount _asglobal_variables) 4))
  (Variables|/Script/Engine.CharacterMovementComponent|SetMaxWalkSpeed (Variables|Character|GetCharacterMovement) (Variables|Default|GetMaxWalkSpeed)))

(event Collision|EventActorBeginOverlap
  (params (OtherActor :type Actor%20Object%20Reference))
  (if (not (Actor|ActorHasTag OtherActor "lightAttack"))
    (bind _asbp_top_down_character (Utilities|Casting|CastToBP_TopDownCharacter OtherActor))
    (Game|Damage|ApplyDamage _asbp_top_down_character 1.0 (Game|GetPlayerController 0) self)
    (Utilities|Time|SetTimerbyFunctionName 0 "DealDamage" 0.5 true)))

(event EventTick
  (params (DeltaSeconds :type Float%20%28single-precision%29))
  (bind _returnvalue (Game|GetPlayerCharacter 0))
  (bind _returnvalue_2 (Transformation|GetActorLocation _returnvalue))
  (if (not (Variables|Default|GetisBeingHIt))
    (AI|AIMoveTo self (Math|Vector|MakeVector (.x _returnvalue_2) (.y _returnvalue_2) 0.0) 0 5.0 true)))

(event Game|Damage|EventAnyDamage
  (params (Damage :type Float%20%28single-precision%29) (DamageType :type Damage%20Type%20Object%20Reference) (InstigatedBy :type Controller%20Object%20Reference) (DamageCauser :type Actor%20Object%20Reference))
  (bind _returnvalue (Math|Random|RandomInteger 8))
  (Sprite|SetSpriteColor (Variables|Default|GetfatBat_Flipbook) "(R=1.000000,G=0.000000,B=0.000000,A=1.000000)")
  (Audio|PlaySoundatLocation "/Game/Sound/Attack/impact_a.impact_a" (Transformation|GetActorLocation) "0, 0, 0" 1.0 1.0 0.0 0 0 0 0)
  (bind _output_get (Variables|Default|SetHealth (- (Variables|Default|GetHealth) Damage)))
  (if (<= _output_get 0)
    (Actor|DestroyActor)
    (bind _asglobal_variables (Utilities|Casting|CastToglobalVariables (Game|GetGameInstance)))
    (Variables|/Game/Blueprints/globalVariables.globalVariables_C|SetremainingEnemies _asglobal_variables (- (Variables|/Game/Blueprints/globalVariables.globalVariables_C|GetremainingEnemies _asglobal_variables) 1))
    (if (== (Math|Random|RandomInteger 2) 1)
      (if (== _returnvalue 1)
        (Game|SpawnActorfromClass :Class "/Game/TopDown/Blueprints/UI/Inventory/PlaceholderUntilBetterSystem/BP_CocktailItem.BP_CocktailItem_C" :SpawnTransform (Math|Transform|MakeTransform (.location (Transformation|GetActorTransform)) "0, 0, 0" "1.000000,1.000000,1.000000") :CollisionHandlingOverride "Undefined" :TransformScaleMethod "MultiplyWithRoot" :Instigator 0)
        (elif (== _returnvalue 2)
          (Game|SpawnActorfromClass :Class "/Game/TopDown/Blueprints/UI/Inventory/PlaceholderUntilBetterSystem/BP_CoffeeItem.BP_CoffeeItem_C" :SpawnTransform (Math|Transform|MakeTransform (.location (Transformation|GetActorTransform)) "0, 0, 0" "1.000000,1.000000,1.000000") :CollisionHandlingOverride "Undefined" :TransformScaleMethod "MultiplyWithRoot" :Instigator 0)
          (elif (== _returnvalue 3)
            (Game|SpawnActorfromClass :Class "/Game/TopDown/Blueprints/UI/Inventory/PlaceholderUntilBetterSystem/BP_FirepokerItem.BP_FirepokerItem_C" :SpawnTransform (Math|Transform|MakeTransform (.location (Transformation|GetActorTransform)) "0, 0, 0" "1.000000,1.000000,1.000000") :CollisionHandlingOverride "Undefined" :TransformScaleMethod "MultiplyWithRoot" :Instigator 0)
            (elif (== _returnvalue 4)
              (Game|SpawnActorfromClass :Class "/Game/TopDown/Blueprints/UI/Inventory/PlaceholderUntilBetterSystem/BP_HatItem.BP_HatItem_C" :SpawnTransform (Math|Transform|MakeTransform (.location (Transformation|GetActorTransform)) "0, 0, 0" "1.000000,1.000000,1.000000") :CollisionHandlingOverride "Undefined" :TransformScaleMethod "MultiplyWithRoot" :Instigator 0)
              (elif (== _returnvalue 5)
                (Game|SpawnActorfromClass :Class "/Game/TopDown/Blueprints/UI/Inventory/PlaceholderUntilBetterSystem/BP_OilcanItem.BP_OilcanItem_C" :SpawnTransform (Math|Transform|MakeTransform (.location (Transformation|GetActorTransform)) "0, 0, 0" "1.000000,1.000000,1.000000") :CollisionHandlingOverride "Undefined" :TransformScaleMethod "MultiplyWithRoot" :Instigator 0)
                (elif (== _returnvalue 6)
                  (Game|SpawnActorfromClass :Class "/Game/TopDown/Blueprints/UI/Inventory/PlaceholderUntilBetterSystem/BP_TicketItem.BP_TicketItem_C" :SpawnTransform (Math|Transform|MakeTransform (.location (Transformation|GetActorTransform)) "0, 0, 0" "1.000000,1.000000,1.000000") :CollisionHandlingOverride "Undefined" :TransformScaleMethod "MultiplyWithRoot" :Instigator 0)
                  (elif (== _returnvalue 7)
                    (Game|SpawnActorfromClass :Class "/Game/TopDown/Blueprints/UI/Inventory/PlaceholderUntilBetterSystem/BP_WatchItem.BP_WatchItem_C" :SpawnTransform (Math|Transform|MakeTransform (.location (Transformation|GetActorTransform)) "0, 0, 0" "1.000000,1.000000,1.000000") :CollisionHandlingOverride "Undefined" :TransformScaleMethod "MultiplyWithRoot" :Instigator 0)
                    (elif (== _returnvalue 8)
                      (Game|SpawnActorfromClass :Class "/Game/TopDown/Blueprints/UI/Inventory/PlaceholderUntilBetterSystem/BP_WhistleItme.BP_WhistleItme_C" :SpawnTransform (Math|Transform|MakeTransform (.location (Transformation|GetActorTransform)) "0, 0, 0" "1.000000,1.000000,1.000000") :CollisionHandlingOverride "Undefined" :TransformScaleMethod "MultiplyWithRoot" :Instigator 0))))))))))
    (else
      (Variables|/Script/Engine.CharacterMovementComponent|SetMaxWalkSpeed (Variables|Character|GetCharacterMovement) 5e+01)
      (Utilities|FlowControl|Delay 0.2)
      (Sprite|SetSpriteColor (Variables|Default|GetfatBat_Flipbook) "(R=1.000000,G=1.000000,B=1.000000,A=1.000000)")
      (Variables|/Script/Engine.CharacterMovementComponent|SetMaxWalkSpeed (Variables|Character|GetCharacterMovement) 1e+02))))

(event Collision|EventActorEndOverlap
  (params (OtherActor :type Actor%20Object%20Reference))
  (if (not (Actor|ActorHasTag OtherActor "lightAttack"))
    (Utilities|FlowControl|Delay 0.2)
    (Utilities|Time|ClearTimerbyFunctionName 0 "DealDamage")))

(fn ConstructionScript)