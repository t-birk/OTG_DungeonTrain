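; Spawner actor that releases EmberEnemy instances at its own transform, with a total count that scales with the current level.
; On BeginPlay it multiplies a base count by LevelCount from the globalVariables game instance and starts a looping one-second timer.
; Each tick of the timer spawns one enemy while the count remains and the player is beyond a distance threshold, with debug prints tracking progress.
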(event Custom|ember_spawn
  (Development|PrintString (Utilities|String|ToString(Integer) (Variables|Default|GetspawnCount)))
  (if (> (Variables|Default|GetspawnCount) 0)
    (if (> (Transformation|GetDistanceTo (Game|GetPlayerCharacter 0)) 1e+03)
      (Game|SpawnActorfromClass "/Game/Blueprints/EmberEnemy.EmberEnemy_C" (Transformation|GetActorTransform) "Undefined" "MultiplyWithRoot" 0 0)
      (bind _output_get (Variables|Default|SetspawnCount (- (Variables|Default|GetspawnCount) 1)))
      (Development|PrintString "SPAWNER IS LOOPING")
      (Development|PrintString (Utilities|String|ToString(Integer) _output_get)))))

(event EventBeginPlay
  (Variables|Default|SetspawnCount 10)
  (bind _asglobal_variables (Utilities|Casting|CastToglobalVariables (Game|GetGameInstance)))
  (bind _output_get (Variables|Default|SetspawnCount (* (Variables|/Game/Blueprints/globalVariables.globalVariables_C|GetlevelCount _asglobal_variables) (Variables|Default|GetspawnCount))))
  (Development|PrintString (Utilities|String|ToString(Integer) _output_get))
  (Utilities|Time|SetTimerbyFunctionName 0 "ember_spawn" 1.0 true))

(fn ConstructionScript)