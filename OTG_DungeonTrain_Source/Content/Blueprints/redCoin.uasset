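; Red coin pickup actor that drifts toward the player and adds to the red money count when collected.
; Entering MagnetizeAOE starts a looping timer that offsets the coin along the normalized direction to the player; leaving clears it.
; Any overlap with the inner Sphere increments RedMoneyCount on the globalVariables game instance, destroys the coin and plays the coin sound at world origin.
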(event OnComponentBeginOverlap(MagnetizeAOE)
  (params (OverlappedComponent :type Primitive%20Component%20Object%20Reference) (OtherActor :type Actor%20Object%20Reference) (OtherComp :type Primitive%20Component%20Object%20Reference) (OtherBodyIndex :type Integer) (bFromSweep :type Boolean) (SweepResult :type Hit%20Result%20Structure%20%28by%20ref%29))
  (if (== OtherActor (Game|GetPlayerCharacter 0))
    (Variables|Default|SetTarget%20Actor OtherActor)
    (Utilities|Time|SetTimerbyEvent (delegate Custom|PullTowardsPlayer) 0.01 true)))

(event OnComponentBeginOverlap(Sphere)
  (params (OverlappedComponent :type Primitive%20Component%20Object%20Reference) (OtherActor :type Actor%20Object%20Reference) (OtherComp :type Primitive%20Component%20Object%20Reference) (OtherBodyIndex :type Integer) (bFromSweep :type Boolean) (SweepResult :type Hit%20Result%20Structure%20%28by%20ref%29))
  (bind _asglobal_variables (Utilities|Casting|CastToglobalVariables (Game|GetGameInstance)))
  (bind _result (Math|Integer|IncrementInt (Variables|/Game/Blueprints/globalVariables.globalVariables_C|GetredMoneyCount _asglobal_variables))
    (:%20%20
      (Variables|/Game/Blueprints/globalVariables.globalVariables_C|SetredMoneyCount _asglobal_variables _result)
      (Actor|DestroyActor)
      (Audio|PlaySoundatLocation "/Game/Sound/coin.coin" "0, 0, 0" "0, 0, 0" 1.0 1.0 0.0 0 0 0 0))))

(event OnComponentEndOverlap(MagnetizeAOE)
  (params (OverlappedComponent :type Primitive%20Component%20Object%20Reference) (OtherActor :type Actor%20Object%20Reference) (OtherComp :type Primitive%20Component%20Object%20Reference) (OtherBodyIndex :type Integer))
  (if (== OtherActor (Game|GetPlayerCharacter 0))
    (Variables|Default|SetTarget%20Actor 0)
    (Utilities|Time|ClearTimerbyFunctionName 0 "PullTowardsPlayer")))

(event Custom|PullTowardsPlayer
  (Transformation|AddActorLocalOffset (* (Math|Vector|Normalize (- (Transformation|GetActorLocation (Variables|Default|GetTarget%20Actor)) (Transformation|GetActorLocation))) (Utilities|Time|GetWorldDeltaSeconds) (Variables|Default|GetSpeed)) false false))

(event EventBeginPlay)

(fn ConstructionScript)