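; Enemy bat actor that moves diagonally on the XY plane and bounces off what it hits.
; BeginPlay picks a random sign for the X and Y velocity, and Tick feeds that vector to the BatMovement component as input.
; On Hit it prints a debug message and flips Y if the hit location's Y differs from the actor's, otherwise X if that differs, using exact float comparisons.
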(event EventBeginPlay
  (Variables|Default|SetbatVelocity (Math|Vector|MakeVector (select (Math|Random|RandomBool) 1.0 -1.0) (select (Math|Random|RandomBool) 1.0 -1.0) 0.0)))

(event Collision|EventHit
  (params (MyComp :type Primitive%20Component%20Object%20Reference) (Other :type Actor%20Object%20Reference) (OtherComp :type Primitive%20Component%20Object%20Reference) (bSelfMoved :type Boolean) (HitLocation :type Vector :default "0, 0, 0") (HitNormal :type Vector :default "0, 0, 0") (NormalImpulse :type Vector :default "0, 0, 0") (Hit :type Hit%20Result%20Structure%20%28by%20ref%29))
  (bind _self self)
  (bind _returnvalue (Transformation|GetActorLocation _self))
  (Development|PrintText "Hit")
  (if (!= (.y _returnvalue) (.y HitLocation))
    (Variables|Default|SetbatVelocity (Math|Vector|MakeVector (.x (Variables|Default|GetbatVelocity)) (* (.y (Variables|Default|GetbatVelocity)) -1.0) (.z (Variables|Default|GetbatVelocity))))
    (elif (!= (.x HitLocation) (.x _returnvalue))
      (Variables|Default|SetbatVelocity (Math|Vector|MakeVector (* (.x (Variables|Default|GetbatVelocity)) -1.0) (.y (Variables|Default|GetbatVelocity)) (.z (Variables|Default|GetbatVelocity)))))))

(event EventTick
  (params (DeltaSeconds :type Float%20%28single-precision%29))
  (Class|PawnMovementComponent|AddInputVector (Variables|Default|GetbatMovement) (Variables|Default|GetbatVelocity) false))

(fn ConstructionScript)