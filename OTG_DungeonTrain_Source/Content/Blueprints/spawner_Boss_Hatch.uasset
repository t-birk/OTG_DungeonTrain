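; Spawner actor that creates a Boss_hatch at its own transform on boss levels, meaning every fourth level count, once no enemies remain.
; Each Tick it casts the game instance to globalVariables and checks RemainingEnemies and LevelCount.
; It has no one-shot guard of its own, so it spawns again on every frame while both conditions hold.
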(event EventBeginPlay)

(event Collision|EventActorBeginOverlap
  (params (OtherActor :type Actor%20Object%20Reference)))

(event EventTick
  (params (DeltaSeconds :type Float%20%28single-precision%29))
  (bind _asglobal_variables (Utilities|Casting|CastToglobalVariables (Game|GetGameInstance)))
  (if (and (== (Variables|/Game/Blueprints/globalVariables.globalVariables_C|GetremainingEnemies _asglobal_variables) 0) (== (Math|Integer|%(Integer) (Variables|/Game/Blueprints/globalVariables.globalVariables_C|GetlevelCount _asglobal_variables) 4) 0))
    (Game|SpawnActorfromClass "/Game/Blueprints/boss_hatch.boss_hatch_C" (Transformation|GetActorTransform) "Undefined" "MultiplyWithRoot" 0 0)))

(fn ConstructionScript)