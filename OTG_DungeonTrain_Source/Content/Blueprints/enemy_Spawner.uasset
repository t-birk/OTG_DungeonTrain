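; Enemy spawner actor that releases Enemy_Ember instances at its own location, with the wave size scaled to the current level.
; On BeginPlay it sets the spawn and remaining-enemy counts in the globalVariables GameInstance from LevelCount, then starts a looping timer.
; Each tick of that timer spawns one ember and decrements the shared spawn count, provided spawns remain and the player is far enough away.
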(event Custom|ember_spawn
  (bind _asglobal_variables (Utilities|Casting|CastToglobalVariables (Game|GetGameInstance)))
  (if (> (Variables|/Game/Blueprints/globalVariables.globalVariables_C|GetspawnCount _asglobal_variables) 0)
    (if (> (Transformation|GetDistanceTo (Game|GetPlayerCharacter 0)) 1e+03)
      (Game|SpawnActorfromClass "/Game/Blueprints/enemy_Ember.enemy_Ember_C" (Transformation|GetActorTransform) "Undefined" "MultiplyWithRoot" 0 0)
      (bind _asglobal_variables_2 (Utilities|Casting|CastToglobalVariables (Game|GetGameInstance)))
      (Variables|/Game/Blueprints/globalVariables.globalVariables_C|SetspawnCount _asglobal_variables_2 (- (Variables|/Game/Blueprints/globalVariables.globalVariables_C|GetspawnCount _asglobal_variables_2) 1))
      (Development|PrintString "Spawn Count")
      (Development|PrintString (Utilities|String|ToString(Integer) (- (Variables|/Game/Blueprints/globalVariables.globalVariables_C|GetspawnCount _asglobal_variables_2) 1))))))

(event EventBeginPlay
  (bind _asglobal_variables (Utilities|Casting|CastToglobalVariables (Game|GetGameInstance)))
  (Variables|/Game/Blueprints/globalVariables.globalVariables_C|SetspawnCount _asglobal_variables (* (Variables|/Game/Blueprints/globalVariables.globalVariables_C|GetlevelCount _asglobal_variables) 10))
  (bind _output_get (Variables|/Game/Blueprints/globalVariables.globalVariables_C|SetremainingEnemies _asglobal_variables (* (Variables|/Game/Blueprints/globalVariables.globalVariables_C|GetlevelCount _asglobal_variables) 10)))
  (Development|PrintString "TOTAL ENEMIES:")
  (Development|PrintString (Utilities|String|ToString(Integer) _output_get))
  (Utilities|Time|SetTimerbyFunctionName 0 "ember_spawn" 4.0 true))

(fn ConstructionScript)