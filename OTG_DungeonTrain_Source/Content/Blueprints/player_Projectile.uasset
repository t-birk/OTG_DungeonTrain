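; Player projectile that damages Ember enemies on contact.
; On actor overlap it casts the game instance to globalVariables and the other actor to enemy_Ember, ignoring any other actor.
; It prints the instance's AttackPower to screen, applies it as damage with the first player controller as instigator, then destroys itself.
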(event EventBeginPlay)

(event Collision|EventActorBeginOverlap
  (params (OtherActor :type Actor%20Object%20Reference))
  (bind _asglobal_variables (Utilities|Casting|CastToglobalVariables (Game|GetGameInstance)))
  (bind _asenemy_ember (Utilities|Casting|CastToenemy_Ember OtherActor))
  (Development|PrintString (Utilities|String|ToString(Float) (* (Variables|/Game/Blueprints/globalVariables.globalVariables_C|GetattackPower _asglobal_variables) 1.0)))
  (Game|Damage|ApplyDamage _asenemy_ember (* (Variables|/Game/Blueprints/globalVariables.globalVariables_C|GetattackPower _asglobal_variables) 1.0) (Game|GetPlayerController 0) self)
  (Actor|DestroyActor))

(event EventTick
  (params (DeltaSeconds :type Float%20%28single-precision%29)))

(fn ConstructionScript)