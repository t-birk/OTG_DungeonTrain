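; EmberEnemy is an enemy actor that homes in on the player and destroys itself on contact.
; Each Tick it steps a fixed distance along the normalized direction to player character 0, independent of delta time, with its height pinned.
; Overlapping BP_TopDownCharacter calls Collision, which applies OutputDamage to that player before self-destructing.
; Its TakeDamage function subtracts from Health and destroys the actor when none remains.
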(event EventBeginPlay)

(event Collision|EventActorBeginOverlap
  (params (OtherActor :type Actor%20Object%20Reference))
  (if (== (Utilities|GetClass OtherActor) "/Game/TopDown/Blueprints/BP_TopDownCharacter.BP_TopDownCharacter_C")
    (CallFunction|Collision)))

(event EventTick
  (params (DeltaSeconds :type Float%20%28single-precision%29))
  (bind _returnvalue (Transformation|GetActorLocation))
  (bind _returnvalue_2 (Game|GetPlayerCharacter 0))
  (bind _returnvalue_3 (Transformation|GetActorLocation _returnvalue_2))
  (bind _returnvalue_4 (- _returnvalue_3 _returnvalue))
  (bind _returnvalue_5 (Math|Vector|Normalize _returnvalue_4))
  (bind _returnvalue_6 (* _returnvalue_5 3.0))
  (bind _returnvalue_7 (+ _returnvalue _returnvalue_6))
  (Transformation|SetActorLocation (Math|Vector|MakeVector (.x _returnvalue_7) (.y _returnvalue_7) 1e+02) false false))

(fn ConstructionScript)

(fn TakeDamage
  (params (Damage :type Integer))
  (bind _output_get (Variables|Default|SetHealth (- (Variables|Default|GetHealth) Damage)))
  (if (<= _output_get 0)
    (Actor|DestroyActor)))

(fn Collision
  (bind _asbp_top_down_character (Utilities|Casting|CastToBP_TopDownCharacter (Game|GetPlayerCharacter 0)))
  (Default|TakeDamage _asbp_top_down_character (Variables|Default|GetOutputDamage))
  (Actor|DestroyActor))