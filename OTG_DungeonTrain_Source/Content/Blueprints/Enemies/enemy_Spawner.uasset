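; Enemy spawner actor that releases a level-scaled wave of Golems, Embers, Greasemen and Bees at its own location.
; BeginPlay sets the spawn and remaining-enemy totals on the globalVariables GameInstance from LevelCount, then starts a looping timer with an interval randomized once.
; Each tick with budget left and the player far enough away decrements SpawnCount and picks the enemy by modulo priority, defaulting to Bee.
; Greaseman spawns become Bees in the TrainCar level.
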(event Custom|spawn%20Golem
  (Game|SpawnActorfromClass "/Game/Blueprints/Enemies/Golem/enemy_Golem.enemy_Golem_C" (Transformation|GetActorTransform) "Undefined" "MultiplyWithRoot" 0 0))

(event Custom|spawn%20ember
  (Game|SpawnActorfromClass "/Game/Blueprints/Enemies/Ember/enemy_Ember.enemy_Ember_C" (Transformation|GetActorTransform) "Undefined" "MultiplyWithRoot" 0 0))

(event Custom|spawn%20Greaseman
  (bind _returnvalue (Game|GetCurrentLevelName true))
  (if (Utilities|Enum|Equal(Enum) _returnvalue "TrainCar")
    (CallFunction|SpawnBee)
    (else
      (Game|SpawnActorfromClass "/Game/Blueprints/GreasemanEnemy.GreasemanEnemy_C" (Transformation|GetActorTransform) "Undefined" "MultiplyWithRoot" 0 0))))

(event Custom|spawn%20Bee
  (Game|SpawnActorfromClass "/Game/Blueprints/Enemies/Bees/enemy_Bee.enemy_Bee_C" (Transformation|GetActorTransform) "Undefined" "MultiplyWithRoot" 0 0))

(event Custom|spawnEnemy
  (bind _asglobal_variables (Utilities|Casting|CastToglobalVariables (Game|GetGameInstance)))
  (if (> (Variables|/Game/Blueprints/globalVariables.globalVariables_C|GetspawnCount _asglobal_variables) 0)
    (if (> (Transformation|GetDistanceTo (Game|GetPlayerCharacter 0)) 1e+03)
      (if true
        (Variables|/Game/Blueprints/globalVariables.globalVariables_C|SetspawnCount _asglobal_variables (- (Variables|/Game/Blueprints/globalVariables.globalVariables_C|GetspawnCount _asglobal_variables) 1))
        (Development|PrintString "Spawn Count")
        (Development|PrintString (Utilities|String|ToString(Integer) (- (Variables|/Game/Blueprints/globalVariables.globalVariables_C|GetspawnCount _asglobal_variables) 1)))
        (if (== (Math|Integer|%(Integer) (Variables|/Game/Blueprints/globalVariables.globalVariables_C|GetspawnCount _asglobal_variables) 10) 0)
          (CallFunction|SpawnGolem)
          (elif (== (Math|Integer|%(Integer) (Variables|/Game/Blueprints/globalVariables.globalVariables_C|GetspawnCount _asglobal_variables) 3) 0)
            (CallFunction|SpawnEmber)
            (elif (== (Math|Integer|%(Integer) (Variables|/Game/Blueprints/globalVariables.globalVariables_C|GetspawnCount _asglobal_variables) 11) 0)
              (CallFunction|SpawnGreaseman)
              (else
                (CallFunction|SpawnBee)))))))))

(event EventBeginPlay
  (bind _asglobal_variables (Utilities|Casting|CastToglobalVariables (Game|GetGameInstance)))
  (Variables|/Game/Blueprints/globalVariables.globalVariables_C|SetspawnCount _asglobal_variables (* (Variables|/Game/Blueprints/globalVariables.globalVariables_C|GetlevelCount _asglobal_variables) 15))
  (bind _output_get (Variables|/Game/Blueprints/globalVariables.globalVariables_C|SetremainingEnemies _asglobal_variables (* (Variables|/Game/Blueprints/globalVariables.globalVariables_C|GetlevelCount _asglobal_variables) 15)))
  (Development|PrintString "TOTAL ENEMIES:")
  (Development|PrintString (Utilities|String|ToString(Integer) _output_get))
  (Utilities|Time|SetTimerbyFunctionName 0 "spawnEnemy" (Math|Random|RandomFloatinRange 3.0 5.0) true))

(fn ConstructionScript)