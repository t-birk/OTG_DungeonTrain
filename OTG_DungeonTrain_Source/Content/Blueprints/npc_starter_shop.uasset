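; Shopkeeper NPC that sells four randomly picked stat items, with costs randomized and scaled by level count after the first level.
; On BeginPlay it rolls stock, costs and icons and creates a hidden shop widget.
; Overlap toggles a speech bubble, Interact opens or closes the shop, and walking away closes it, with timers sequencing flipbook animations.
; PurchaseItem calls the matching item actor and deducts gold from the GameInstance.
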(event Custom|wave_sprite
  (if (not (Variables|Default|GetinAnimation))
    (if (not (Variables|Default|GetshopIsOpen))
      (Sprite|SetFlipbook (Variables|Default|GetShopkeep) "/Game/2D_Sprites/Shopkeeper/Idle_2/Idle_2_Flipbook.Idle_2_Flipbook")
      (Utilities|FlowControl|Delay (Class|PaperFlipbookComponent|GetFlipbookLength (Variables|Default|GetShopkeep)))
      (Sprite|SetFlipbook (Variables|Default|GetShopkeep) "/Game/2D_Sprites/Shopkeeper/Idle/Idle_1.Idle_1"))))

(event Custom|switch_to_dialogue_idle
  (if (Variables|Default|GetinAnimation)
    (if (not (Variables|Default|GetactivelyClosing))
      (Sprite|SetFlipbook (Variables|Default|GetShopkeep) "/Game/2D_Sprites/Shopkeeper/Dialogue/Dialogue_Idle_Shop.Dialogue_Idle_Shop")
      (Variables|Default|SetinAnimation false))))

(event Custom|switch_to_idle
  (if (Variables|Default|GetinAnimation)
    (Sprite|SetFlipbook (Variables|Default|GetShopkeep) "/Game/2D_Sprites/Shopkeeper/Idle/Idle_1.Idle_1")
    (Variables|Default|SetinAnimation false)))

(event EventBeginPlay
  (CallFunction|GetItemCosts)
  (CallFunction|SetAllItems)
  (Effects|SpawnEmitteratLocation "/Game/StarterContent/Particles/P_Explosion.P_Explosion" (Transformation|GetActorLocation))
  (Utilities|Time|SetTimerbyFunctionName 0 "wave_sprite" 8.0 true)
  (bind _returnvalue (UserInterface|CreateWidget "/Game/TopDown/Blueprints/UI/Shopkeeper/shop_Widget.shop_Widget_C"))
  (Variables|Default|SetshopWidget _returnvalue)
  (UserInterface|Viewport|AddtoViewport _returnvalue 0)
  (Widget|SetVisibility (Variables|Default|GetshopWidget) "Collapsed"))

(event Collision|EventActorBeginOverlap
  (params (OtherActor :type Actor%20Object%20Reference))
  (if (not (Actor|ActorHasTag OtherActor "lightAttack"))
    (if (not (Actor|ActorHasTag OtherActor "heavyAttack"))
      (Rendering|SetVisibility (Variables|Default|GetSpeech%20Bubble) true false))))

(event Collision|EventActorEndOverlap
  (params (OtherActor :type Actor%20Object%20Reference))
  (if (not (Variables|Default|GetactivelyClosing))
    (if (not (Actor|ActorHasTag OtherActor "lightAttack"))
      (if (not (Actor|ActorHasTag OtherActor "heavyAttack"))
        (Rendering|SetVisibility (Variables|Default|GetSpeech%20Bubble) false false)
        (Utilities|FlowControl|Delay 0.5)
        (if (Variables|Default|GetshopIsOpen)
          (Development|PrintString "ping")
          (Variables|Default|SetactivelyClosing true)
          (CallFunction|ShopClose))))))

(event EventInteract
  (if (not (Variables|Default|GetinAnimation))
    (if (Variables|Default|GetshopIsOpen)
      (CallFunction|ShopClose)
      (elif (not (Variables|Default|GetactivelyClosing))
        (if (not (Variables|Default|GetinAnimation))
          (CallFunction|ShopOpen))))))

(fn ConstructionScript)

(fn ShopClose
  (bind _shopkeep (Variables|Default|GetShopkeep))
  (Variables|Default|SetactivelyClosing true)
  (Widget|SetVisibility (Variables|Default|GetshopWidget) "Collapsed")
  (Variables|Default|SetinAnimation true)
  (Sprite|SetFlipbook _shopkeep "/Game/2D_Sprites/Shopkeeper/Dialogue/Dialogue_Close_Shop.Dialogue_Close_Shop")
  (Utilities|Time|SetTimerbyFunctionName 0 "switch_to_idle" (- (Class|PaperFlipbookComponent|GetFlipbookLength _shopkeep) 0.1) false true)
  (Variables|Default|SetactivelyClosing false)
  (Variables|Default|SetshopIsOpen false))

(fn ShopOpen
  (bind _shopkeep (Variables|Default|GetShopkeep))
  (Widget|SetVisibility (Variables|Default|GetshopWidget) "Visible")
  (Variables|Default|SetinAnimation true)
  (Sprite|SetFlipbook _shopkeep "/Game/2D_Sprites/Shopkeeper/Dialogue/Dialogue_Open_Shop.Dialogue_Open_Shop")
  (if (not (Variables|Default|GetactivelyClosing))
    (Utilities|Time|SetTimerbyFunctionName 0 "switch_to_dialogue_idle" (Class|PaperFlipbookComponent|GetFlipbookLength _shopkeep) false true)
    (Variables|Default|SetshopIsOpen true)))

(fn GetItemCosts
  (bind _asglobal_variables (Utilities|Casting|CastToglobalVariables (Game|GetGameInstance)))
  (if (> (Variables|/Game/Blueprints/globalVariables.globalVariables_C|GetlevelCount _asglobal_variables) 1)
    (Utilities|FlowControl|Sequence
      (:then_0
        (Variables|Default|SetItem_Cost_1 (Math|Float|Truncate (+ (* (Variables|/Game/Blueprints/globalVariables.globalVariables_C|GetlevelCount _asglobal_variables) (Math|Random|RandomFloatinRange 0.5 (Variables|Default|GetcostModifier))) 2e+01))))
      (:then_1
        (Variables|Default|SetItem_Cost_2 (Math|Float|Truncate (+ (* (Variables|/Game/Blueprints/globalVariables.globalVariables_C|GetlevelCount _asglobal_variables) (Math|Random|RandomFloatinRange 0.5 (Variables|Default|GetcostModifier))) 2e+01))))
      (:then_2
        (Variables|Default|SetItem_Cost_3 (Math|Float|Truncate (+ (* (Variables|/Game/Blueprints/globalVariables.globalVariables_C|GetlevelCount _asglobal_variables) (Math|Random|RandomFloatinRange 0.5 (Variables|Default|GetcostModifier))) 2e+01))))
      (:then_3
        (Variables|Default|SetItem_Cost_4 (Math|Float|Truncate (+ (* (Variables|/Game/Blueprints/globalVariables.globalVariables_C|GetlevelCount _asglobal_variables) (Math|Random|RandomFloatinRange 0.5 (Variables|Default|GetcostModifier))) 2e+01)))))))

(fn GetItems
  (Variables|Default|SetrandomInteger (Math|Random|RandomIntegerinRange 1 8))
  (Development|PrintString (Utilities|String|ToString(Integer) (Variables|Default|GetrandomInteger)))
  (if (== (Variables|Default|GetrandomInteger) 1)
    (Variables|Default|Setavailable_Item "Whistle")
    (Utilities|FlowControl|Sequence :!label _label
      (:then_0
        (return (Variables|Default|Getavailable_item))))
    (elif (== (Variables|Default|GetrandomInteger) 2)
      (Variables|Default|Setavailable_Item "Cocktail")
      (goto _label)
      (elif (== (Variables|Default|GetrandomInteger) 3)
        (Variables|Default|Setavailable_Item "Coffee")
        (goto _label)
        (elif (== (Variables|Default|GetrandomInteger) 4)
          (Variables|Default|Setavailable_Item "Firepoker")
          (goto _label)
          (elif (== (Variables|Default|GetrandomInteger) 5)
            (Variables|Default|Setavailable_Item "Hat")
            (goto _label)
            (elif (== (Variables|Default|GetrandomInteger) 6)
              (Variables|Default|Setavailable_Item "Oil_can")
              (goto _label)
              (elif (== (Variables|Default|GetrandomInteger) 7)
                (Variables|Default|Setavailable_Item "Ticket")
                (goto _label)
                (elif (== (Variables|Default|GetrandomInteger) 8)
                  (Variables|Default|Setavailable_Item "Watch")
                  (goto _label)
                  (else
                    (Development|PrintString "Failed to Set Item String")))))))))))

(fn SetTexture
  (params (Item :type String))
  (Development|PrintString Item)
  (if (Utilities|Enum|Equal(Enum) Item "Whistle")
    (Variables|Default|SetTexture (Class|WidgetBlueprintLibrary|MakeBrushfromTexture "/Game/TopDown/Blueprints/UI/Inventory/Images/Train_Whistle_-_Dash_Charge.Train_Whistle_-_Dash_Charge"))
    (return (Variables|Default|GetTexture))
    (elif (Utilities|Enum|Equal(Enum) Item "Cocktail")
      (Variables|Default|SetTexture (Class|WidgetBlueprintLibrary|MakeBrushfromTexture "/Game/TopDown/Blueprints/UI/Inventory/Images/Cocktail_-_Regen.Cocktail_-_Regen"))
      (return (Variables|Default|GetTexture))
      (elif (Utilities|Enum|Equal(Enum) Item "Coffee")
        (Variables|Default|SetTexture (Class|WidgetBlueprintLibrary|MakeBrushfromTexture "/Game/TopDown/Blueprints/UI/Inventory/Images/Coffee_-_Move_Speed.Coffee_-_Move_Speed"))
        (return (Variables|Default|GetTexture))
        (elif (Utilities|Enum|Equal(Enum) Item "Firepoker")
          (Variables|Default|SetTexture (Class|WidgetBlueprintLibrary|MakeBrushfromTexture "/Game/TopDown/Blueprints/UI/Inventory/Images/Firepoker_-_Attack_.Firepoker_-_Attack_"))
          (return (Variables|Default|GetTexture))
          (elif (Utilities|Enum|Equal(Enum) Item "Hat")
            (Variables|Default|SetTexture (Class|WidgetBlueprintLibrary|MakeBrushfromTexture "/Game/TopDown/Blueprints/UI/Inventory/Images/Conductor_Hat_-_Health.Conductor_Hat_-_Health"))
            (return (Variables|Default|GetTexture))
            (elif (Utilities|Enum|Equal(Enum) Item "Oil_can")
              (Variables|Default|SetTexture (Class|WidgetBlueprintLibrary|MakeBrushfromTexture "/Game/TopDown/Blueprints/UI/Inventory/Images/Oil_Can_-_Attack_Speed.Oil_Can_-_Attack_Speed"))
              (return (Variables|Default|GetTexture))
              (elif (Utilities|Enum|Equal(Enum) Item "Ticket")
                (Variables|Default|SetTexture (Class|WidgetBlueprintLibrary|MakeBrushfromTexture "/Game/TopDown/Blueprints/UI/Inventory/Images/Ticket_-_Dodge_Chance.Ticket_-_Dodge_Chance"))
                (return (Variables|Default|GetTexture))
                (elif (Utilities|Enum|Equal(Enum) Item "Watch")
                  (Variables|Default|SetTexture (Class|WidgetBlueprintLibrary|MakeBrushfromTexture "/Game/TopDown/Blueprints/UI/Inventory/Images/Watch_-_Health.Watch_-_Health"))
                  (return (Variables|Default|GetTexture)))))))))))

(fn SetAllItems
  (Utilities|FlowControl|Sequence
    (:then_0
      (bind _item (CallFunction|GetItems))
      (bind _texture (CallFunction|SetTexture _item))
      (Variables|Default|SetItem_Texture_1 _texture)
      (Variables|Default|SetItem _item))
    (:then_1
      (bind _item_2 (CallFunction|GetItems))
      (bind _texture_2 (CallFunction|SetTexture _item_2))
      (Variables|Default|SetItem_Texture_2 _texture_2)
      (Variables|Default|SetItem_0 _item_2))
    (:then_2
      (bind _item_3 (CallFunction|GetItems))
      (bind _texture_3 (CallFunction|SetTexture _item_3))
      (Variables|Default|SetItem_Texture_3 _texture_3)
      (Variables|Default|SetItem_1 _item_3))
    (:then_3
      (bind _item_4 (CallFunction|GetItems))
      (bind _texture_4 (CallFunction|SetTexture _item_4))
      (Variables|Default|SetItem_Texture_4 _texture_4)
      (Variables|Default|SetItem_2 _item_4))))

(fn PurchaseItem
  (params (Item :type String) (Item%20Cost :type Integer))
  (if (Utilities|Enum|Equal(Enum) Item "Whistle")
    (bind _returnvalue (Actor|GetActorOfClass "/Game/Blueprints/Items/BP_WhistleItem.BP_WhistleItem_C"))
    (Default|AddWhistle _returnvalue)
    (bind _asglobal_variables (Utilities|Casting|CastToglobalVariables (Game|GetGameInstance) :!label _label))
    (Variables|/Game/Blueprints/globalVariables.globalVariables_C|SetgoldMoneyCount _asglobal_variables (- (Variables|/Game/Blueprints/globalVariables.globalVariables_C|GetgoldMoneyCount _asglobal_variables) Item%20Cost))
    (elif (Utilities|Enum|Equal(Enum) Item "Cocktail")
      (bind _returnvalue_2 (Actor|GetActorOfClass "/Game/Blueprints/Items/BP_CocktailItem.BP_CocktailItem_C"))
      (Default|AddCocktail _returnvalue_2)
      (goto _label)
      (elif (Utilities|Enum|Equal(Enum) Item "Coffee")
        (bind _returnvalue_3 (Actor|GetActorOfClass "/Game/Blueprints/Items/BP_CoffeeItem.BP_CoffeeItem_C"))
        (Default|AddCoffee _returnvalue_3)
        (goto _label)
        (elif (Utilities|Enum|Equal(Enum) Item "Firepoker")
          (bind _returnvalue_4 (Actor|GetActorOfClass "/Game/Blueprints/Items/BP_FirepokerItem.BP_FirepokerItem_C"))
          (Default|AddFirepoker _returnvalue_4)
          (goto _label)
          (elif (Utilities|Enum|Equal(Enum) Item "Hat")
            (bind _returnvalue_5 (Actor|GetActorOfClass "/Game/Blueprints/Items/BP_HatItem.BP_HatItem_C"))
            (Default|AddHat _returnvalue_5)
            (goto _label)
            (elif (Utilities|Enum|Equal(Enum) Item "Oil_can")
              (bind _returnvalue_6 (Actor|GetActorOfClass "/Game/Blueprints/Items/BP_OilcanItem.BP_OilcanItem_C"))
              (Default|AddOilCan _returnvalue_6)
              (goto _label)
              (elif (Utilities|Enum|Equal(Enum) Item "Ticket")
                (bind _returnvalue_7 (Actor|GetActorOfClass "/Game/Blueprints/Items/BP_TicketItem.BP_TicketItem_C"))
                (Default|AddTicket _returnvalue_7)
                (goto _label)
                (elif (Utilities|Enum|Equal(Enum) Item "Watch")
                  (bind _returnvalue_8 (Actor|GetActorOfClass "/Game/Blueprints/Items/BP_WatchItem.BP_WatchItem_C"))
                  (Default|AddWatch _returnvalue_8)
                  (goto _label))))))))))