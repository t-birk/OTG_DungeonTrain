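; GreasemanEnemy is a flipbook-animated enemy that periodically fires a projectile at the player.
; On BeginPlay, three looping timers with staggered initial delays switch to the attack flipbook, spawn the projectile, then restore the default flipbook.
; SpawnProjectile creates a GreasemanProjectile at the enemy's location facing the player character, then zeroes its root component's world rotation.
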(event EventBeginPlay
  (Utilities|Time|SetTimerbyFunctionName 0 "FlipbookAttackStart" 3.0 true false 2.9)
  (Utilities|Time|SetTimerbyFunctionName 0 "SpawnProjectile" 3.0 true false 3.15)
  (Utilities|Time|SetTimerbyFunctionName 0 "FlipbookAttackEnd" 3.0 true false 3.3))

(event Collision|EventActorBeginOverlap
  (params (OtherActor :type Actor%20Object%20Reference)))

(event EventTick
  (params (DeltaSeconds :type Float%20%28single-precision%29)))

(fn ConstructionScript)

(fn SpawnProjectile
  (bind _returnvalue (Transformation|GetActorLocation))
  (bind _returnvalue_2 (Game|SpawnActorfromClass "/Game/Blueprints/GreasemanProjectile.GreasemanProjectile_C" (Math|Transform|MakeTransform _returnvalue (Math|Rotator|FindLookatRotation _returnvalue (Transformation|GetActorLocation (Game|GetPlayerCharacter 0))) "1.000000,1.000000,1.000000") "Undefined" "MultiplyWithRoot" 0 0))
  (Transformation|SetWorldRotation (Variables|/Script/Engine.Actor|GetRootComponent _returnvalue_2) "0, 0, 0" false false))

(fn FlipbookAttackEnd
  (Sprite|SetFlipbook (Variables|Default|GetGreaseman_Flipbook) "/Game/2D_Sprites/enemies/grease_frames/grease_flipbook.grease_flipbook"))

(fn FlipbookAttackStart
  (Sprite|SetFlipbook (Variables|Default|GetGreaseman_Flipbook) "/Game/2D_Sprites/enemies/greaseman/greaseman_attack.greaseman_attack"))