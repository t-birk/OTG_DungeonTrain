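; Final boss character with flipbook visuals that chases the player, attacks by range and plays a death sequence at exactly zero HP.
; Tick drives movement animation, AI chasing, a mid-range Sweep that jumps to the player's saved position, and a closer SpinSlam available during Sweep's cooldown.
; HitBox overlap triggers a timer-repeated Slam.
; Attacks share an IsAttacking lock and spawn short-lived damage actors, timed with delays.
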(event OnComponentBeginOverlap(HitBox)
  (params (OverlappedComponent :type Primitive%20Component%20Object%20Reference) (OtherActor :type Actor%20Object%20Reference) (OtherComp :type Primitive%20Component%20Object%20Reference) (OtherBodyIndex :type Integer) (bFromSweep :type Boolean) (SweepResult :type Hit%20Result%20Structure%20%28by%20ref%29))
  (if (not (Actor|ActorHasTag OtherActor "lightAttack"))
    (if (not (Actor|ActorHasTag OtherActor "heavyAttack"))
      (if (not (Actor|ActorHasTag OtherActor "player_Projectile"))
        (CallFunction|Slam)
        (Utilities|Time|SetTimerbyFunctionName 0 "slam" 0.5 true)))))

(event OnComponentEndOverlap(HitBox)
  (params (OverlappedComponent :type Primitive%20Component%20Object%20Reference) (OtherActor :type Actor%20Object%20Reference) (OtherComp :type Primitive%20Component%20Object%20Reference) (OtherBodyIndex :type Integer))
  (if (not (Actor|ActorHasTag OtherActor "lightAttack"))
    (if (not (Actor|ActorHasTag OtherActor "heavyAttack"))
      (if (not (Actor|ActorHasTag OtherActor "player_Projectile"))
        (Utilities|FlowControl|Delay 0.2)
        (Utilities|Time|ClearTimerbyFunctionName 0 "slam")))))

(event OnComponentBeginOverlap(Player_In_Range_Detector)
  (params (OverlappedComponent :type Primitive%20Component%20Object%20Reference) (OtherActor :type Actor%20Object%20Reference) (OtherComp :type Primitive%20Component%20Object%20Reference) (OtherBodyIndex :type Integer) (bFromSweep :type Boolean) (SweepResult :type Hit%20Result%20Structure%20%28by%20ref%29))
  (Development|PrintString "In Range of Boss"))

(event EventBeginPlay
  (Sprite|SetFlipbook (Variables|Default|GetFinalBoss_Flipbook) "/Game/FinalBoss/Shock_Sweeper/Shuffle_Walk/shuffe_move.shuffe_move")
  (Variables|/Script/Engine.CharacterMovementComponent|SetMaxWalkSpeed (Variables|Character|GetCharacterMovement) (Variables|Default|GetMaxWalkSpeed))
  (Variables|Default|SetcurrentHP (Variables|Default|GetmaxHP))
  (Variables|Default|SetbossDead false))

(event EventSpinSlam
  (bind _returnvalue (Game|GetPlayerCharacter 0))
  (bind _returnvalue_2 (Transformation|GetDistanceTo _returnvalue))
  ;[1 1 1] Attacks
  (if (not (Variables|Default|GetbossDead))
    (if (not (Variables|Default|GetisAttacking))
      (if (Variables|Default|GetsweepCooldown)
        (if (not (Variables|Default|GetspinSlamCooldown))
          (if (and (<= _returnvalue_2 4e+02) (>= _returnvalue_2 2e+02))
            (Variables|Default|SetisAttacking true)
            (Components|Activation|Deactivate (Variables|Character|GetCharacterMovement))
            (Utilities|FlowControl|Delay 0.2)
            (Sprite|SetFlipbook (Variables|Default|GetFinalBoss_Flipbook) "/Game/FinalBoss/Shock_Sweeper/Spin_Slam/Spin_Slam_with_VFX1.Spin_Slam_with_VFX1")
            (Utilities|FlowControl|Sequence
              (:then_0
                (Utilities|FlowControl|Delay 1.1)
                (Sprite|SetFlipbook (Variables|Default|GetFinalBoss_Flipbook) "/Game/FinalBoss/Shock_Sweeper/static_idle_Flipbook.static_idle_Flipbook")
                (Variables|Default|SetisAttacking false)
                (Components|Activation|Activate (Variables|Character|GetCharacterMovement) false)
                (Variables|Default|SetspinSlamCooldown true)
                (Utilities|FlowControl|Delay 5.0)
                (Variables|Default|SetspinSlamCooldown false))
              (:then_1
                (Utilities|FlowControl|Delay 0.4)
                (Audio|PlaySoundatLocation "/Game/StarterContent/Audio/Explosion01.Explosion01" (Transformation|GetActorLocation) "0, 0, 0" 1.0 1.0 0.0 0 0 0 0)
                (bind _returnvalue_3 (Game|SpawnActorfromClass "/Game/FinalBoss/boss_AOE_attack.boss_AOE_attack_C" (Transformation|GetActorTransform) "Undefined" "MultiplyWithRoot" 0 0))
                (Utilities|FlowControl|Delay 0.2)
                (Actor|DestroyActor _returnvalue_3)))))))))

(event EventTick
  (params (DeltaSeconds :type Float%20%28single-precision%29))
  (bind _returnvalue (Game|GetPlayerCharacter 0))
  (bind _returnvalue_2 (Transformation|GetVelocity))
  (bind _returnvalue_3 (Transformation|GetVelocity))
  (bind _returnvalue_4 (Transformation|GetActorLocation _returnvalue))
  (Utilities|FlowControl|Sequence
    (:then_0
      (CallFunction|SpinSlam))
    (:then_1
      (if (not (Variables|Default|GetisAttacking))
        (if (!= (.y _returnvalue_3) 0.0)
          (Sprite|SetFlipbook (Variables|Default|GetFinalBoss_Flipbook) "/Game/FinalBoss/Shock_Sweeper/Shuffle_Walk/shuffe_move.shuffe_move")
          (if (< (.y _returnvalue_3) 0.0)
            (Transformation|SetRelativeScale3D (Variables|Default|GetFinalBoss_Flipbook) "6.500000,6.500000,6.500000")
            (elif (> (.y _returnvalue_3) 0.0)
              (Transformation|SetRelativeScale3D (Variables|Default|GetFinalBoss_Flipbook) "-6.500000,6.500000,6.500000"))))))
    (:then_2
      (if (and (== (.y _returnvalue_2) 0.0) (== (.x _returnvalue_2) 0.0))
        (if (not (Variables|Default|GetbossDead))
          (if (not (Variables|Default|GetisAttacking))
            (Sprite|SetFlipbook (Variables|Default|GetFinalBoss_Flipbook) "/Game/FinalBoss/Shock_Sweeper/static_idle_Flipbook.static_idle_Flipbook")))))
    (:then_3
      (if (not (Variables|Default|GetbossDead))
        (if (not (Variables|Default|GetisAttacking))
          (AI|AIMoveTo self (Math|Vector|MakeVector (.x _returnvalue_4) (.y _returnvalue_4) 0.0) (Game|GetPlayerCharacter 0) 5.0 true))))
    (:then_4
      (CallFunction|Sweep))))

(event Game|Damage|EventAnyDamage
  (params (Damage :type Float%20%28single-precision%29) (DamageType :type Damage%20Type%20Object%20Reference) (InstigatedBy :type Controller%20Object%20Reference) (DamageCauser :type Actor%20Object%20Reference))
  ;[1 1 1] Taking Damage
  (Sprite|SetSpriteColor (Variables|Default|GetFinalBoss_Flipbook) "(R=1.000000,G=0.000000,B=0.000000,A=1.000000)")
  (bind _output_get (Variables|Default|SetcurrentHP (- (Variables|Default|GetcurrentHP) Damage)))
  (Audio|PlaySoundatLocation "/Game/Sound/Attack/impact_a.impact_a" (Transformation|GetActorLocation) "0, 0, 0" 1.0 1.0 0.0 0 0 0 0)
  (Utilities|FlowControl|Delay 0.2)
  (Sprite|SetSpriteColor (Variables|Default|GetFinalBoss_Flipbook) "(R=1.000000,G=1.000000,B=1.000000,A=1.000000)")
  (if (== _output_get 0.0)
    (Components|Movement|StopMovementImmediately (Variables|Character|GetCharacterMovement))
    (Components|Activation|Deactivate (Variables|Character|GetCharacterMovement))
    (Variables|Default|SetbossDead true)
    (Utilities|FlowControl|Delay 0.5)
    (Sprite|SetFlipbook (Variables|Default|GetFinalBoss_Flipbook) "/Game/FinalBoss/Shock_Sweeper/Death/death1.death1")
    (Utilities|FlowControl|Delay 0.45)
    (Sprite|SetFlipbook (Variables|Default|GetFinalBoss_Flipbook) "/Game/FinalBoss/Shock_Sweeper/Death/death2.death2")))

(event EventSweep
  (bind _returnvalue (Game|GetPlayerCharacter 0))
  (bind _returnvalue_2 (Transformation|GetDistanceTo _returnvalue))
  ;[1 1 1] Attacks
  (if (and (<= _returnvalue_2 8e+02) (>= _returnvalue_2 4.5e+02))
    (Variables|Default|SetPlayerLocation (Transformation|GetActorLocation (Game|GetPlayerCharacter 0)))
    (if (not (Variables|Default|GetbossDead))
      (if (Variables|Default|GetisAttacking)
        (Development|PrintString "waaa")
        (elif (not (Variables|Default|GetsweepCooldown))
          (Variables|Default|SetisAttacking true)
          (Utilities|FlowControl|Sequence
            (:then_0
              (Utilities|FlowControl|Delay 1.0)
              (Sprite|SetFlipbook (Variables|Default|GetFinalBoss_Flipbook) "/Game/FinalBoss/Shock_Sweeper/Sweep/Sweep_with_VFX1.Sweep_with_VFX1")
              (Transformation|SetRelativeLocation (Variables|Collision|GetCapsuleComponent) (Math|Vector|Lerp(Vector) (Variables|Default|GetPlayerLocation) (Transformation|GetActorLocation) 0.0) true false)
              (Audio|PlaySoundatLocation "/Game/Sound/Attack/woosh_a.woosh_a" (Transformation|GetActorLocation) "0, 0, 0" 0.5 1.0 0.0 0 0 0 0)
              (Utilities|FlowControl|Sequence
                (:then_0
                  (Utilities|FlowControl|Delay 1.15)
                  (Sprite|SetFlipbook (Variables|Default|GetFinalBoss_Flipbook) "/Game/FinalBoss/Shock_Sweeper/static_idle_Flipbook.static_idle_Flipbook")
                  (Variables|Default|SetisAttacking false)
                  (Variables|Default|SetsweepCooldown true)
                  (Utilities|FlowControl|Delay 3.0)
                  (Variables|Default|SetsweepCooldown false))
                (:then_1
                  (Utilities|FlowControl|Delay 0.6)
                  (bind _returnvalue_3 (Game|SpawnActorfromClass "/Game/FinalBoss/boss_Basic_Attack.boss_Basic_Attack_C" (Transformation|GetActorTransform) "Undefined" "MultiplyWithRoot" 0 0))
                  (Utilities|FlowControl|Delay 0.2)
                  (Actor|DestroyActor _returnvalue_3))))
            (:then_1
              (Audio|PlaySoundatLocation "/Engine/EditorSounds/GamePreview/StartPlayInEditor.StartPlayInEditor" (Transformation|GetActorLocation) "0, 0, 0" 1.0 1.0 0.0 0 0 0 0))))))))

(event EventSlam
  ;[1 1 1] Attacks
  (if (not (Variables|Default|GetbossDead))
    (if (not (Variables|Default|GetisAttacking))
      (Variables|Default|SetisAttacking true)
      (Components|Activation|Deactivate (Variables|Character|GetCharacterMovement))
      (bind _output_get (Variables|Default|SetPlayerTransform (Transformation|GetActorTransform)))
      (Sprite|SetFlipbook (Variables|Default|GetFinalBoss_Flipbook) "/Game/FinalBoss/Shock_Sweeper/Slam/slam_with_VFX1.slam_with_VFX1")
      (Utilities|FlowControl|Delay 1.0)
      (bind _returnvalue (Game|SpawnActorfromClass "/Game/FinalBoss/boss_Basic_Attack.boss_Basic_Attack_C" _output_get "Undefined" "MultiplyWithRoot" 0 0))
      (Utilities|FlowControl|Delay 0.2)
      (Actor|DestroyActor _returnvalue)
      (Sprite|SetFlipbook (Variables|Default|GetFinalBoss_Flipbook) "/Game/FinalBoss/Shock_Sweeper/Shuffle_Walk/shuffe_move.shuffe_move")
      (Variables|Default|SetisAttacking false)
      (Components|Activation|Activate (Variables|Character|GetCharacterMovement) false))))

(fn ConstructionScript)